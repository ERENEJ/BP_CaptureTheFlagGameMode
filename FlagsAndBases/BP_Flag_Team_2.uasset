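; Team 2 (Militia) capture-the-flag flag, which enemy soldiers pick up and teammates return to base.
; On box overlap, the server attaches the flag to a living enemy's head socket or resets it to its pole for a teammate.
; A fast looping timer polls the carrier and drops the flag in place on death.
; Take, drop and return events multicast a widget notification and sound.
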(event OnComponentBeginOverlap(Box)
  (params (OverlappedComponent :type Primitive%20Component%20Object%20Reference) (OtherActor :type Actor%20Object%20Reference) (OtherComp :type Primitive%20Component%20Object%20Reference) (OtherBodyIndex :type Integer) (bFromSweep :type Boolean) (SweepResult :type Hit%20Result%20Structure%20%28by%20ref%29))
  (Networking|SwitchHasAuthority
    (:Authority
      ;[1 1 1] Decides flag movement if it is gonna attach to player or returns the base
      (if (not (Variables|Default|GetIsFlagCarried))
        (bind _assqsoldier (Utilities|Casting|CastToSQSoldier OtherActor))
        (if (Class|SQSoldier|IsAlive _assqsoldier)
          (if (!= (Class|SQSoldier|GetTeam _assqsoldier) (Variables|Default|GetTeamIndex))
            (if (not (Variables|Default|GetIsFlagCarried))
              ;[1 1 1] Attaches flag to soldier
              (Networking|SwitchHasAuthority
                (:Authority
                  (Transformation|AttachComponentToComponent (Variables|Default|GetStaticMesh) (Variables|/Script/Engine.Character|GetMesh _assqsoldier) "Bip01_Head" "SnapToTarget" "KeepWorld" "SnapToTarget" false)
                  (Actor|SetOwner _assqsoldier)
                  (bind _assqsoldier_2 (Utilities|Casting|CastToSQSoldier (Components|GetOwner)))
                  (bind _returnvalue (Utilities|Time|SetTimerbyEvent (delegate Custom|SR_CheckFlagCarrier) 0.02 true))
                  (Variables|Default|SetFlagInBase false)
                  (Variables|Default|SetIsFlagCarried true)
                  (CallFunction|SRShowFlagInfo "Milita flag taken!"))))
            (elif (not (Variables|Default|GetIsFlagCarried))
              ;[1 1 1] RESETS FLAG
              (Development|PrintString "FLAG RESETED!")
              (Networking|SwitchHasAuthority
                (:Authority
                  (CallFunction|SRResetFlag)))))
          (else
            (Variables|Default|SetIsFlagCarried false)))))))

(event Custom|SR_ShowFlagInfo
  (params (FlagInfoName :type Text))
  ;[0 0.1602 1 1 26] TODO UI PART  is valid part added later
  (CallFunction|MultiSetandShowFlagInfo FlagInfoName))

(event Custom|SR_CheckFlagCarrier
  ;[1 1 1] Check flag carrier health and drops flag when flag carrier is dead
  (Networking|SwitchHasAuthority
    (:Authority
      (CallFunction|CheckFlagCarrier (stale OnComponentBeginOverlap(Box) _assqsoldier_2)))))

(event Custom|Multi_SetAndShowFlagInfo
  (params (FlagInfoName :type Text))
  ;[0 0.1602 1 1 26] TODO UI PART  is valid part added later
  (bind _outactors (Actor|GetAllActorsOfClass "/Game/Blueprints/BP_PlayerController.BP_PlayerController_C"))
  (for _array_element _outactors
    (bind _returnvalue (UserInterface|CreateWidget "/CapturetheFlagGameMode/TopFolder/BP_CtFMainWidget.BP_CtFMainWidget_C" _array_element))
    (bind _returnvalue_2 (UserInterface|CreateWidget "/CapturetheFlagGameMode/TopFolder/W_FlagInfoMessage.W_FlagInfoMessage_C"))
    (Default|SetFlagNotification _returnvalue_2 FlagInfoName)
    (Widget|Panel|AddChild (Variables|/CapturetheFlagGameMode/TopFolder/BP_CtFMainWidget.BP_CtFMainWidget_C|GetNotificationBox _returnvalue) _returnvalue_2)
    (UserInterface|Viewport|AddtoViewport _returnvalue 0)
    (Audio|PlaySound2D "/CapturetheFlagGameMode/TopFolder/VO_US_SL_Gratitudute_placeholder_PlaceHolder.VO_US_SL_Gratitudute_placeholder_PlaceHolder" 1.0 1.0 0.0 0 0)
    (Utilities|FlowControl|Delay 3.0)))

(event Custom|CheckFlagCarrier
  (params (Target :type SQ%20Soldier%20Object%20Reference))
  ;[1 1 1] Check flag carrier health and drops flag when flag carrier is dead
  (if (not (Class|SQSoldier|IsAlive Target))
    (Variables|Default|SetIsFlagCarried false)
    (Transformation|DetachFromComponent (Variables|Default|GetStaticMesh) "KeepWorld" "KeepWorld" "KeepWorld" true)
    (Variables|Default|SetCurrentFlagPosition (+ "0, 0,20.000000" (Transformation|GetWorldLocation (Variables|Default|GetStaticMesh))))
    (Transformation|SetWorldLocationAndRotation (Variables|Default|GetStaticMesh) (Variables|Default|GetCurrentFlagPosition) "0, 0, 0" false false)
    (Utilities|Time|ClearandInvalidateTimerbyHandle (stale OnComponentBeginOverlap(Box) _returnvalue))
    (CallFunction|SRShowFlagInfo "Milita flag dropped!")))

(event Custom|SR_ResetFlag
  ;[1 1 1] RESETS FLAG
  (if (not (Variables|Default|GetFlagInBase))
    (Transformation|AttachComponentToComponent (Variables|Default|GetStaticMesh) (Variables|Default|Getafgpole04) "" "SnapToTarget" "SnapToTarget" "SnapToTarget" true)
    (Variables|Default|SetFlagInBase true)
    (Variables|Default|SetIsFlagCarried false)
    (CallFunction|SRShowFlagInfo "Milita flag returned the base")))

(fn ConstructionScript)