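; Team 1 flag base for capture-the-flag that scores when an actor carrying the Team 2 flag enters its sphere.
; On server overlap it finds the attached enemy flag, checks that Team 1's flag is in base within the sphere, and deducts Team 2 tickets.
; It then respawns the captured flag at its recorded capture position and multicasts a notification widget and sound to player controllers.
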(event OnComponentBeginOverlap(Sphere1)
  (params (OverlappedComponent :type Primitive%20Component%20Object%20Reference) (OtherActor :type Actor%20Object%20Reference) (OtherComp :type Primitive%20Component%20Object%20Reference) (OtherBodyIndex :type Integer) (bFromSweep :type Boolean) (SweepResult :type Hit%20Result%20Structure%20%28by%20ref%29))
  (Networking|SwitchHasAuthority
    (:Authority
      (CallFunction|SRCheckFlagBase OtherActor))))

(event Custom|SR_CheckFlagBase
  (params (OtherOverlapedActor :type Actor%20Object%20Reference))
  (bind (_outteamstate _returnvalue) (Class|SQGameplayService|TryGetTeamState 2))
  ;[1 1 1] Checks for flags and sets score
  (for _array_element (Actor|GetAttachedActors OtherOverlapedActor)
    (bind _asbp_flag_team_2 (Utilities|Casting|CastToBP_Flag_Team_2 _array_element))
    (bind _output_get (Variables|Default|SetBP_Flag_NEWTeam_2 _asbp_flag_team_2))
    (Variables|Default|SetFlagPosition (Transformation|GetActorLocation _output_get))
    (Development|PrintString "Flag in zone" true true "(R=0.000000,G=0.660000,B=1.000000,A=1.000000)" 5.0)
    (if _returnvalue
      (for _array_element_2 (Collision|GetOverlappingActors (Variables|Default|GetSphere1) 0 :!class /Script/Engine.PrimitiveComponent)
        (bind _asbp_flag_team_1 (Utilities|Casting|CastToBP_Flag_Team_1 _array_element_2))
        (if (Variables|/CapturetheFlagGameMode/TopFolder/FlagsAndBases/BP_Flag_Team_1.BP_Flag_Team_1_C|GetFlagInBase _asbp_flag_team_1)
          (Variables|/Script/Squad.SQTeamState|SetTickets _outteamstate (- (Variables|/Script/Squad.SQTeamState|GetTickets _outteamstate) 50))
          (Networking|SwitchHasAuthority
            (:Authority
              (CallFunction|SRResetCappedFlag))))))))

(event Custom|SR_ShowFlagInfo
  (params (FlagInfoName :type Text))
  ;[0 0.1602 1 1 26] TODO UI PART
  (CallFunction|MultiSetandShowFlagInfo FlagInfoName))

(event Custom|Multi_SetAndShowFlagInfo
  (params (FlagInfoName :type Text))
  ;[0 0.1602 1 1 26] TODO UI PART
  (bind _outactors (Actor|GetAllActorsOfClass "/Game/Blueprints/BP_PlayerController.BP_PlayerController_C"))
  (for _array_element _outactors
    (bind _returnvalue (UserInterface|CreateWidget "/CapturetheFlagGameMode/TopFolder/BP_CtFMainWidget.BP_CtFMainWidget_C" _array_element))
    (bind _returnvalue_2 (UserInterface|CreateWidget "/CapturetheFlagGameMode/TopFolder/W_FlagInfoMessage.W_FlagInfoMessage_C"))
    (Default|SetFlagNotification _returnvalue_2 FlagInfoName)
    (Widget|Panel|AddChild (Variables|/CapturetheFlagGameMode/TopFolder/BP_CtFMainWidget.BP_CtFMainWidget_C|GetNotificationBox _returnvalue) _returnvalue_2)
    (UserInterface|Viewport|AddtoViewport _returnvalue 0)
    (Audio|PlaySound2D "/CapturetheFlagGameMode/TopFolder/VO_US_SL_Gratitudute_placeholder_PlaceHolder.VO_US_SL_Gratitudute_placeholder_PlaceHolder" 1.0 1.0 0.0 0 0)
    (Utilities|FlowControl|Delay 3.0)))

(event Custom|Multi_CheckFlagBase
  (params (OtherOverlapedActor :type Actor%20Object%20Reference)))

(event Custom|SR_ResetCappedFlag
  ;[1 1 1] Respawns flag after the score
  (Actor|DestroyActor (Variables|Default|GetBP_Flag_NEWTeam_2))
  (bind _returnvalue (Game|SpawnActorfromClass "/CapturetheFlagGameMode/TopFolder/FlagsAndBases/BP_Flag_Team_2.BP_Flag_Team_2_C" (Math|Transform|MakeTransform (Variables|Default|GetFlagPosition) "0, 0, 0" "1,1,1") "AlwaysSpawn" 0 2 0))
  (bind _output_get (Variables|Default|SetBP_Flag_NEWTeam_2 _returnvalue))
  (Variables|/CapturetheFlagGameMode/TopFolder/FlagsAndBases/BP_Flag_Team_2.BP_Flag_Team_2_C|SetIsFlagCarried _output_get false)
  (Transformation|AttachComponentToComponent (Variables|/CapturetheFlagGameMode/TopFolder/FlagsAndBases/BP_Flag_Team_2.BP_Flag_Team_2_C|GetStaticMesh (Variables|Default|GetBP_Flag_NEWTeam_2)) (Variables|/CapturetheFlagGameMode/TopFolder/FlagsAndBases/BP_Flag_Team_2.BP_Flag_Team_2_C|Getafgpole04 (Variables|Default|GetBP_Flag_NEWTeam_2)) "" "SnapToTarget" "KeepWorld" "KeepWorld" true)
  (CallFunction|SRShowFlagInfo "Team1 Capped the flag!"))

(fn ConstructionScript)