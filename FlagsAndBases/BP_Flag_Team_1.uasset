(event OnComponentBeginOverlap(Box)
  (params (OverlappedComponent :type Primitive%20Component%20Object%20Reference) (OtherActor :type Actor%20Object%20Reference) (OtherComp :type Primitive%20Component%20Object%20Reference) (OtherBodyIndex :type Integer) (bFromSweep :type Boolean) (SweepResult :type Hit%20Result%20Structure%20%28by%20ref%29))
  ;[1 1 1] Decides flag movement if it is gonna attach to player or returns the base
  (Networking|SwitchHasAuthority
    (:Authority
      (if (not (Variables|Default|GetIsFlagCarried))
        (bind _assqsoldier (Utilities|Casting|CastToSQSoldier OtherActor))
        (if (Class|SQSoldier|IsAlive _assqsoldier)
          (if (!= (Class|SQSoldier|GetTeam _assqsoldier) (Variables|Default|GetTeamIndex))
            (if (not (Variables|Default|GetIsFlagCarried))
              ;[1 1 1] Attaches flag to soldier
              (Networking|SwitchHasAuthority
                (:Authority
                  (Transformation|AttachComponentToComponent (Variables|Default|GetStaticMesh) (Variables|/Script/Engine.Character|GetMesh _assqsoldier) "Bip01_HeadNub" "SnapToTarget" "KeepWorld" "SnapToTarget" false)
                  (Actor|SetOwner _assqsoldier)
                  (bind _assqsoldier_2 (Utilities|Casting|CastToSQSoldier (Components|GetOwner)))
                  (Variables|Default|SetFlagInBase false)
                  (Variables|Default|SetIsFlagCarried true)
                  (CallFunction|SRShowFlagInfo " flag taken!" (Variables|Default|GetTeamIndex) (Utilities|Array|Get(acopy) (Variables|Default|GetTFlagSoundsArray) 1))
                  (bind _returnvalue (Utilities|Time|SetTimerbyEvent (delegate Custom|SR_CheckFlagCarrier) 0.02 true)))))
            (elif (not (Variables|Default|GetIsFlagCarried))
              ;[1 1 1] RESETS FLAG
              (Development|PrintString "FLAG RESETED!")
              (Networking|SwitchHasAuthority
                (:Authority
                  (CallFunction|SRResetFlag)))))
          (else
            (Variables|Default|SetIsFlagCarried false)))))))

(event Custom|SR_ShowFlagInfo
  (params (FlagInfoName :type Text) (TeamIndex :type Integer%20%28by%20ref%29) (FlagNotificationSıund :type Sound%20Wave%20Object%20Reference%20%28by%20ref%29))
  ;[0 0.1602 1 1 26] UI PART There is a room for upgrade
  (CallFunction|MultiSetandShowFlagInfo FlagInfoName TeamIndex FlagNotificationSıund))

(event Custom|SR_CheckFlagCarrier
  ;[1 1 1] Check flag carrier health and drops flag when flag carrier is dead
  (Networking|SwitchHasAuthority
    (:Authority
      (CallFunction|CheckFlagCarrier (stale OnComponentBeginOverlap(Box) _assqsoldier_2)))))

(event Custom|Multi_SetAndShowFlagInfo
  (params (FlagInfoName :type Text) (TeamIndex :type Integer%20%28by%20ref%29) (FlagNotificationSound :type Sound%20Wave%20Object%20Reference%20%28by%20ref%29))
  (bind _outteamconfig (Class|SQSettingsService|TryGetLocalPlayerTeamLayerConfig))
  ;[0 0.1602 1 1 26] UI PART There is a room for upgrade
  (bind _outactors (Actor|GetAllActorsOfClass "/Game/Blueprints/BP_PlayerController.BP_PlayerController_C"))
  (for _array_element _outactors
    (Utilities|IsValid _outteamconfig
      (:Is%20Valid
        (if (== (Math|Conversions|ToByte(Integer) TeamIndex) (Variables|/Script/Squad.SQLayerTeamConfig|GetIndex _outteamconfig))
          (Variables|Default|SetPronounOfPlayer (Utilities|Text|FormatText "Your{FlagInfoName}" FlagInfoName))
          (Audio|PlaySound2D FlagNotificationSound 0.6 1.0 0.0 0 0)
          (else
            (Variables|Default|SetPronounOfPlayer (Utilities|Text|FormatText "Enemy{FlagInfoName}" FlagInfoName))
            (Audio|PlaySound2D FlagNotificationSound 0.6 0.125 0.0 0 0)))
        (bind _returnvalue (UserInterface|CreateWidget "/CapturetheFlagGameMode/TopFolder/BP_CtFMainWidget.BP_CtFMainWidget_C" _array_element))
        (bind _returnvalue_2 (UserInterface|CreateWidget "/CapturetheFlagGameMode/TopFolder/W_FlagInfoMessage.W_FlagInfoMessage_C"))
        (Utilities|IsValid _returnvalue_2
          (:Is%20Valid
            (Default|SetFlagNotification2 _returnvalue_2 (Variables|Default|GetPronounOfPlayer))
            (Utilities|IsValid (Variables|/CapturetheFlagGameMode/TopFolder/BP_CtFMainWidget.BP_CtFMainWidget_C|GetNotificationBox_2 _returnvalue)
              (:Is%20Valid
                (Widget|Panel|AddChild (Variables|/CapturetheFlagGameMode/TopFolder/BP_CtFMainWidget.BP_CtFMainWidget_C|GetNotificationBox_2 _returnvalue) _returnvalue_2)
                (Utilities|IsValid _returnvalue
                  (:Is%20Valid
                    (UserInterface|Viewport|AddtoViewport _returnvalue 0)))))))))))

(event Custom|CheckFlagCarrier
  (params (Target :type SQ%20Soldier%20Object%20Reference))
  ;[1 1 1] Check flag carrier health and drops flag when flag carrier is dead
  (Variables|Default|SetCurrentFlagPosition (Transformation|GetWorldLocation (Variables|Default|GetStaticMesh)))
  (if (not (Class|SQSoldier|IsAlive Target))
    (Variables|Default|SetIsFlagCarried false)
    (Transformation|DetachFromComponent (Variables|Default|GetStaticMesh) "KeepWorld" "KeepWorld" "KeepWorld" true)
    (Variables|Default|SetCurrentFlagPosition (+ "0, 0,20.000000" (Transformation|GetWorldLocation (Variables|Default|GetStaticMesh))))
    (Transformation|SetWorldLocationAndRotation (Variables|Default|GetStaticMesh) (Variables|Default|GetCurrentFlagPosition) "0, 0, 0" false false)
    (Utilities|Time|ClearandInvalidateTimerbyHandle (stale OnComponentBeginOverlap(Box) _returnvalue))
    (CallFunction|SRShowFlagInfo " flag dropped!" (Variables|Default|GetTeamIndex) (Utilities|Array|Get(acopy) (Variables|Default|GetTFlagSoundsArray)))))

(event Custom|SR_ResetFlag
  ;[1 1 1] RESETS FLAG
  (if (not (Variables|Default|GetFlagInBase))
    (Transformation|AttachComponentToComponent (Variables|Default|GetStaticMesh) (Variables|Default|Getafgpole04) "" "SnapToTarget" "SnapToTarget" "SnapToTarget" true)
    (Variables|Default|SetFlagInBase true)
    (Variables|Default|SetIsFlagCarried false)
    (CallFunction|SRShowFlagInfo " flag returned the base!" (Variables|Default|GetTeamIndex) (Utilities|Array|Get(acopy) (Variables|Default|GetTFlagSoundsArray) 2))))

(fn ConstructionScript)