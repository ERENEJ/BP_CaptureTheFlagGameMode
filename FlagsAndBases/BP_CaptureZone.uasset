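; Capture zone actor that gives the local player flag animation and sound feedback when the zone changes team.
; It binds to SQCaptureZone's state-change event on actor overlap, forwarding team changes to a cosmetic-only handler.
; A fog-of-war check on team, capturability or admin camera gates the HUD animation.
; Faction-specific sounds queue through UI_Events_Component if the player is inside, including in vehicle seats, unless disabled in saved settings.
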(event Custom|CaptureStateChangeEvent_Event_0
  (params (CaptureZone :type SQ%20Capture%20Zone%20Component%20Object%20Reference) (Team :type Byte))
  (bind _sqcapturezone (Variables|Default|GetSQCaptureZone))
  (bind _lastowningteam (Variables|/Script/Squad.SQCaptureZoneComponent|GetLastOwningTeam _sqcapturezone))
  (if (!= Team _lastowningteam)
    (CallFunction|MultiCaptureStateChanged Team _lastowningteam)))

(event Custom|Multi%20Capture%20State%20Changed
  (params (Team :type Byte) (LastTeam :type Byte))
  (Networking|CanExecuteCosmeticEvents
    (:True
      (if (CallFunction|FogOfWarCheck)
        (CallFunction|UIFlagAnimation Team LastTeam)
        (Utilities|IsValid (CallFunction|GetUISaveData)
          (:Is%20Valid
            (if (Variables|/Game/UI/SaveData_UI.SaveData_UI_C|GetPlay%20Capture%20Sounds (CallFunction|GetUISaveData))
              (if (CallFunction|IsPlayerinZone) :!label _label
                (CallFunction|PlayCaptureSound (Math|Conversions|ToInteger(Byte) Team) (Math|Conversions|ToInteger(Byte) LastTeam)))))
          (:Is%20Not%20Valid
            (goto _label)))))))

(event EventBeginPlay)

(event Collision|EventActorBeginOverlap
  (params (OtherActor :type Actor%20Object%20Reference))
  (EventDispatchers|AssignCaptureStateChangeEvent (Variables|Default|GetSQCaptureZone) (delegate Custom|CaptureStateChangeEvent_Event_0)))

(fn ConstructionScript)

(fn IsPlayerinZone
  (bind _assqplayer_state (Utilities|Casting|CastToSQPlayerState (Variables|/Script/Engine.Controller|GetPlayerState (Game|GetPlayerController 0))))
  (bind _soldier (Variables|/Script/Squad.SQPlayerState|GetSoldier _assqplayer_state)
    (:then
      (LocalVariables|SetL%20Player%20Soldier _soldier)
      (for _array_element (Collision|GetOverlappingActors "/Script/Engine.Pawn" :!class /Script/Engine.Actor)
        (Utilities|IsValid _array_element
          (:Is%20Valid
            (bind _assqvehicle (Utilities|Casting|CastToSQVehicle _array_element)
              (:then
                (for _array_element_2 (Class|SQVehicle|GetSeats _assqvehicle)
                  (Utilities|IsValid _array_element_2
                    (:Is%20Valid
                      (bind _seatedsoldier (Variables|/Script/Squad.SQVehicleSeatComponent|GetSeatedSoldier _array_element_2)
                        (:then
                          (if (== _seatedsoldier (LocalVariables|GetL%20Player%20Soldier))
                            (return true)))
                        (:else))))))
              (:CastFailed
                (if (== _array_element (LocalVariables|GetL%20Player%20Soldier))
                  (return true))))))))
    (:else)))

(fn FogOfWarCheck
  (bind _assqplayer_controller (Utilities|Casting|CastToSQPlayerController (Game|GetPlayerController 0)))
  (return (Math|Boolean|ORBoolean (== (Math|Conversions|ToInteger(Byte) (Variables|/Script/Squad.SQCaptureZoneComponent|GetOwningTeam (Variables|Default|GetSQCaptureZone))) (Class|SQPlayerController|GetTeam _assqplayer_controller)) (Class|SQCaptureZoneComponent|GetCanTeamCapture (Variables|Default|GetSQCaptureZone) (Math|Conversions|ToByte(Integer) (Class|SQPlayerController|GetTeam _assqplayer_controller))) (Class|SQPlayerController|IsAdminCamera _assqplayer_controller) (Variables|/Script/Squad.SQCaptureZoneComponent|GetUncappable (Variables|Default|GetSQCaptureZone)))))

(fn UIFlagAnimation
  (params (New%20Owning%20Team :type Byte) (Last%20Owning%20Team :type Byte))
  (bind _returnvalue (Game|GetPlayerController 0))
  (bind _returnvalue_2 (HUD|GetHUD _returnvalue))
  (bind _returnvalue_3 (Actor|GetComponentbyClass _returnvalue_2 "/Game/UI/UI_Components/UI_Events_Component.UI_Events_Component_C"))
  (Utilities|IsValid _returnvalue
    (:Is%20Valid
      (Utilities|IsValid _returnvalue_2
        (:Is%20Valid
          (Utilities|IsValid _returnvalue_3
            (:Is%20Valid
              (Default|PlayFlagCaptureAnimation _returnvalue_3 (Variables|Default|GetSQCaptureZone) New%20Owning%20Team Last%20Owning%20Team))))))))

(fn PlayCaptureSound
  (params (New%20Team%20Id :type Integer) (Last%20Team%20Id :type Integer))
  (bind _outfaction (Class|SQSettingsService|TryGetLocalPlayerFaction "/Game/Settings/Factions/BP_SQFaction.BP_SQFaction_C"))
  (bind (_outplayercontroller _returnvalue) (Class|SQGameplayService|TryGetLocalPlayerController))
  (bind (_outteamid _returnvalue_2) (Class|SQGameplayService|TryGetLocalPlayerTeamId))
  (bind _returnvalue_3 (HUD|GetHUD _outplayercontroller))
  (bind _returnvalue_4 (Utilities|GetClass _outfaction))
  (bind (_outfaction_2 _returnvalue_5) (Class|SQSettingsService|TryGetLocalPlayerFaction _returnvalue_4))
  (bind _returnvalue_6 (Actor|GetComponentbyClass _returnvalue_3 "/Game/UI/UI_Components/UI_Events_Component.UI_Events_Component_C"))
  (bind (_success _factionentry) (Default|TryGetFactionEntry _outfaction_2))
  (bind _objectivesounds (Utilities|Struct|BreakSQFactionEntry _factionentry))
  (bind _output (Utilities|Array|Get(acopy) _objectivesounds))
  (if _returnvalue
    (if _returnvalue_2
      (LocalVariables|SetOurTeamIsLast (== _outteamid Last%20Team%20Id))
      (LocalVariables|SetOurTeamIsNew (== _outteamid New%20Team%20Id))
      (Utilities|IsValid _returnvalue_3
        (:Is%20Valid
          (Utilities|IsValid _returnvalue_6
            (:Is%20Valid
              (LocalVariables|SetL%20UI%20Events _returnvalue_6)
              (if _returnvalue_5
                (if _success
                  (if (Utilities|Array|IsValidIndex _objectivesounds)
                    ;[1 1 1] Our Team Neutralized
                    (if (and (not (LocalVariables|GetOurTeamIsLast)) (LocalVariables|GetOurTeamIsNew))
                      (Default|AddSoundtoAsyncQueue (LocalVariables|GetL%20UI%20Events) (.objectivebeingwon _output))
                      (else
                        ;[1 1 1] Flag Being Lost
                        (if (and (LocalVariables|GetOurTeamIsLast) (not (LocalVariables|GetOurTeamIsNew)))
                          (Default|AddSoundtoAsyncQueue (LocalVariables|GetL%20UI%20Events) (.objectivebeinglost _output))
                          (else
                            ;[1 1 1] Flag Capture or Lost
                            (if (LocalVariables|GetOurTeamIsLast)
                              (Default|AddSoundtoAsyncQueue (LocalVariables|GetL%20UI%20Events) (.objectivelost _output))
                              (elif (LocalVariables|GetOurTeamIsNew)
                                (Default|AddSoundtoAsyncQueue (LocalVariables|GetL%20UI%20Events) (.objectivewon _output))))))))))))))))))